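; Level tile actor that fills itself with random props and chains to new tiles as the player advances.
; On BeginPlay it locks its barrier and calls InserisciAttori per container, box, bag and rock type with count, radius and scale ranges.
; The player overlapping NextLevel turns the barrier green and passable; leaving relocks it red.
; CreateDestroy overlap has BPGameMode create a tile and calls VDestroy on this one; GetAttachedArrow exposes the arrow's transform.
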(event `self.ReceiveBeginPlay`
  (`self.Blocco`)
  (`self.InserisciAttori` "/Game/Props/BP_Container_Close.BP_Container_Close_C" 2 4 400.0 1.0 1.0)
  (`self.InserisciAttori` "/Game/Props/BP_Box1.BP_Box1_C" 3 6 200.0 1.0 1.0)
  (`self.InserisciAttori` "/Game/Props/BP_Container_Open.BP_Container_Open_C" 2 4 400.0 1.0 1.0)
  (`self.InserisciAttori` "/Game/Props/BP_Box2.BP_Box2_C" 3 6 200.0 1.0 1.0)
  (`self.InserisciAttori` "/Game/Props/BP_Bags.BP_Bags_C" 4 7 150.0 1.0 1.0)
  (`self.InserisciAttori` "/Game/Props/BP_Rock1.BP_Rock1_C" 2 5 300.0 0.5 2.0)
  (`self.InserisciAttori` "/Game/Props/BP_Box5.BP_Box5_C" 1 3 300.0 1.0 1.0)
  (`self.InserisciAttori` "/Game/Props/BP_Box4.BP_Box4_C" 3 6 300.0 1.0 1.0)
  (`self.InserisciAttori` "/Game/Props/BP_Rock.BP_Rock_C" 4 8 300.0 0.5 2.0)
  (`self.InserisciAttori` "/Game/Props/BP_Rock2.BP_Rock2_C" 4 8 300.0 0.5 2.0))

(event `self.NextLevel.OnComponentEndOverlap`
  (params (OverlappedComponent :type "PrimitiveComponent Object Reference") (OtherActor :type "Actor Object Reference") (OtherComp :type "PrimitiveComponent Object Reference") (OtherBodyIndex :type Integer))
  (`self.Validate` OtherActor)
  (`self.Blocco`))

(event `self.NextLevel.OnComponentBeginOverlap`
  (params (OverlappedComponent :type "PrimitiveComponent Object Reference") (OtherActor :type "Actor Object Reference") (OtherComp :type "PrimitiveComponent Object Reference") (OtherBodyIndex :type Integer) (bFromSweep :type Boolean) (SweepResult :type "HitResult Structure (by ref)"))
  (`self.Validate` OtherActor)
  (`self.Sblocco`))

(event `self.CreateDestroy.OnComponentBeginOverlap`
  (params (OverlappedComponent :type "PrimitiveComponent Object Reference") (OtherActor :type "Actor Object Reference") (OtherComp :type "PrimitiveComponent Object Reference") (OtherBodyIndex :type Integer) (bFromSweep :type Boolean) (SweepResult :type "HitResult Structure (by ref)"))
  (`self.Validate` OtherActor)
  (bind _asbpgame_mode (cast `/Game/Blueprint/Blueprints/BPGameMode` (`GameplayStatics.GetGameMode`)))
  (`ShooterpGameMode.CreaTile` _asbpgame_mode)
  (`ShooterpGameMode.VDestroy` self))

(fn `Blocco`
  (bind _barrier (`self.Barrier`))
  (`PrimitiveComponent.SetCollisionEnabled` _barrier "QueryAndPhysics")
  (`PrimitiveComponent.SetMaterial` _barrier 0 "/Game/Materials/BarrierRed.BarrierRed"))

(fn `GetAttachedArrow`
  (returns (ReturnValue :type "Transform Structure"))
  (return (`SceneComponent.K2_GetComponentToWorld` (`self.Arrow`))))

(fn `Sblocco`
  (bind _barrier (`self.Barrier`))
  (`PrimitiveComponent.SetCollisionEnabled` _barrier "NoCollision")
  (`PrimitiveComponent.SetMaterial` _barrier 0 "/Game/Materials/BarrierGreen.BarrierGreen"))

(fn `UserConstructionScript`)